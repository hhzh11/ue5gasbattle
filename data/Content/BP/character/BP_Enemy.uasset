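; BP_Enemy is an enemy character Blueprint that reacts to health changes and stops its AI on death.
; Its HP change event calls the parent handler, then stops the AI Controller's brain logic if the death flag is set.
; The same event updates an overhead UMG enemy health bar widget with the new value divided by an ability system attribute.
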(event EventBeginPlay)

(event Collision|EventActorBeginOverlap
  (params (OtherActor :type Actor%20Object%20Reference)))

(event EventTick
  (params (DeltaSeconds :type Float%20%28single-precision%29)))

(event EventHPChangeEvent事件
  (params (NewValue :type Float%20%28single-precision%29))
  (|CallParentFunction NewValue)
  (Utilities|FlowControl|Sequence
    (:then_0
      (if (Variables|Default|Getisdeath)
        (CallFunction|Stopai)))
    (:then_1
      (bind _asumg_enemy_bar (Utilities|Casting|CastToUMG_EnemyBar (UserInterface|GetUserWidgetObject (Variables|Default|GetHpBar))))
      (Default|SetBar _asumg_enemy_bar (/ NewValue (.ReturnValue (Ability|Attribute|GetFloatAttributefromAbilitySystemComponent (Variables|Default|GetAbilitySystem) "(AttributeName=\"MaxHP\",Attribute=/Script/roglike_gas.BaseAttributeSet:MaxHP,AttributeOwner=\"/Script/CoreUObject.Class'/Script/roglike_gas.BaseAttributeSet'\")")))))))

(fn ConstructionScript
  (|CallParentFunction))

(fn Stopai
  (bind _asai_controller_0 (Utilities|Casting|CastToAI_Controller0 (Pawn|GetController)))
  (AI|Logic|StopLogic (Variables|/Script/AIModule.AIController|GetBrainComponent _asai_controller_0) "Death"))