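; BP_BaseCharacter is a character base using the Gameplay Ability System for melee combat, health and death.
; BeginPlay disables the hit Capsule's collision, grants GAB_Melee and binds HP changes to a death check.
; Melee activates abilities by indexed tag, and Capsule overlaps apply GE_MeleeDamage to characters of a different class.
; At zero HP it plays the death montage once, and non-player characters grant the player experience through a GameplayEffect.
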(event OnComponentBeginOverlap(Capsule)
  (params (OverlappedComponent :type Primitive%20Component%20Object%20Reference) (OtherActor :type Actor%20Object%20Reference) (OtherComp :type Primitive%20Component%20Object%20Reference) (OtherBodyIndex :type Integer) (bFromSweep :type Boolean) (SweepResult :type Hit%20Result%20Structure%20%28by%20ref%29))
  (if (and (!= OtherActor self) (!= (Utilities|GetClass OtherActor) (Utilities|GetClass self)))
    (bind _asbp_base_character (Utilities|Casting|CastToBP_BaseCharacter OtherActor))
    (GameplayEffects|ApplyGameplayEffectToTarget :self (Variables|Default|GetAbilitySystem) :GameplayEffectClass "/Game/BP/Ability/Melee/GE_MeleeDamage.GE_MeleeDamage_C" :Target (Variables|BP_BaseCharacter_C|GetAbilitySystem _asbp_base_character))))

(event Custom|Melee
  (CallFunction|ActiveAbility))

(event Custom|HPChangeEvent_事件
  (params (NewValue :type Float%20%28single-precision%29))
  (CallFunction|CEIsdeath NewValue))

(event Custom|CE_isdeath
  (params (HP :type Float%20%28double-precision%29))
  (if (and (not (Variables|Default|Getisdeath)) (<= HP 0.0))
    (Variables|Default|Setisdeath true)
    (Animation|Montage|PlayMontage (Variables|Character|GetMesh) "/Game/Ani/Montage/MA_Death.MA_Death"
      (:then
        (Utilities|Casting|CastToBP_Player self
          (:CastFailed
            (GameplayEffects|ApplyGameplayEffectToTarget :self (Variables|Default|GetAbilitySystem) :GameplayEffectClass "/Game/BP/Ability/ExprienceAdd/GE_AddExprience.GE_AddExprience_C" :Target (Variables|BP_BaseCharacter_C|GetAbilitySystem (.Player (CallFunction|GetPlayerandPC))))))))))

(event EventBeginPlay
  (Utilities|FlowControl|Sequence
    (:then_0
      (Collision|SetCollisionEnabled (Variables|Default|GetCapsule) "NoCollision"))
    (:then_1
      (GameplayAbilities|GiveAbility (Variables|Default|GetAbilitySystem) "/Game/BP/Ability/Melee/GAB_Melee.GAB_Melee_C" 0 -1)
      (EventDispatchers|AssignHPChangeEvent (delegate Custom|HPChangeEvent_事件)))))

(event Collision|EventActorBeginOverlap
  (params (OtherActor :type Actor%20Object%20Reference)))

(event EventTick
  (params (DeltaSeconds :type Float%20%28single-precision%29)))

(fn ConstructionScript)

(fn ActiveAbility
  (params (abilityIndex :type Integer))
  (Abilities|TryActivateAbilitiesbyTag (Variables|Default|GetAbilitySystem) (Utilities|Array|Get(acopy) (Variables|Default|GetGameplay%20Tag%20Container) abilityIndex) true))