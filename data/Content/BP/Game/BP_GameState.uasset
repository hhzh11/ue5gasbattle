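; BP_GameState is a game state Blueprint that runs a repeating ten-second countdown to trigger spawning.
; On begin play it resets the timer and calls SpawnActorCustom on the BP_Actor found in the level.
; Tick decrements the timer and writes the clamped, rounded value to the player controller's main UI countdown text.
; When time runs out, Tick restarts the countdown and looks up BP_Actor again to spawn.
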(event EventBeginPlay
  (Variables|Default|SetPrepareTime 1e+01)
  (bind _returnvalue (Actor|GetActorOfClass "/Game/BP/Game/BP_Actor.BP_Actor_C"))
  (Default|SpawnActorCustom _returnvalue))

(event EventTick
  (params (DeltaSeconds :type Float%20%28single-precision%29))
  (if (> (Variables|Default|GetPrepareTime) 0.0)
    (bind _output_get (Variables|Default|SetPrepareTime (- (Variables|Default|GetPrepareTime) DeltaSeconds)))
    (Rendering|Components|TextRender|SetText (Variables|/Game/BP/character/UMG/UMG_mainUI.UMG_mainUI_C|Getcountdowntime (Variables|/Game/BP/Gameplay/BP_PlayerController.BP_PlayerController_C|GetMainUI (.PC (CallFunction|GetPlayerandPC)))) (Utilities|Text|ToText(Float) (Math|Float|Clamp(Float) _output_get 0.0 1e+01) "HalfToEven" false true 1 324 0 0))
    (else
      (Variables|Default|SetPrepareTime 1e+01)
      (bind _returnvalue (Actor|GetActorOfClass "/Game/BP/Game/BP_Actor.BP_Actor_C"))
      (Default|SpawnActorCustom _returnvalue))))

(fn ConstructionScript)